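; Player input actor that tracks the grid tile under the cursor and runs the selected left and right click actions on it.
; Tick updates the hovered state on BP_Grid, and a hover change re-runs the action of any held button, allowing drag application.
; SetSelectedActions replaces both action actors by spawning the given classes with a reference to itself, then broadcasts the change.
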(event Custom|onHoveredTileChange
  (Utilities|FlowControl|Sequence
    (:then_0
      (if (Variables|Default|Getis_left_click_down)
        (Utilities|IsValid (Variables|Default|GetselectedAction_LeftClick)
          (:Is%20Valid
            (Default|ExecAction (Variables|Default|GetselectedAction_LeftClick) (Variables|Default|Gethovered_tile))))))
    (:then_1
      (if (Variables|Default|Getis_right_click_down)
        (Utilities|IsValid (Variables|Default|GetselectedAction_RightClick)
          (:Is%20Valid
            (Default|ExecAction (Variables|Default|GetselectedAction_RightClick) (Variables|Default|Gethovered_tile))))))))

(event EventBeginPlay
  (bind _returnvalue (Actor|GetActorOfClass "/Game/Blueprints/Core/Grid/BP_Grid.BP_Grid_C"))
  (Variables|Default|Setgrid _returnvalue)
  (Input|EnableInput (Game|GetPlayerController 0)))

(event EventTick
  (params (DeltaSeconds :type Float%20%28single-precision%29))
  (CallFunction|UpdateTileUnderCursor))

(event Input|MouseEvents|LeftMouseButton
  (params (Key :type Key%20Structure :default "None"))
  (:Pressed
    (CallFunction|UpdateTileUnderCursor)
    (Variables|Default|Setis_left_click_down true)
    (Utilities|IsValid (Variables|Default|GetselectedAction_LeftClick)
      (:Is%20Valid
        (Default|ExecAction (Variables|Default|GetselectedAction_LeftClick) (Variables|Default|Gethovered_tile)))))
  (:Released
    (Variables|Default|Setis_left_click_down false)))

(event Input|MouseEvents|RightMouseButton
  (params (Key :type Key%20Structure :default "None"))
  (:Pressed
    (CallFunction|UpdateTileUnderCursor)
    (Variables|Default|Setis_right_click_down true)
    (Utilities|IsValid (Variables|Default|GetselectedAction_RightClick)
      (:Is%20Valid
        (Default|ExecAction (Variables|Default|GetselectedAction_RightClick) (Variables|Default|Gethovered_tile)))))
  (:Released
    (Variables|Default|Setis_right_click_down false)))

(fn ConstructionScript)

(fn UpdateTileUnderCursor
  ;[1 1 1] Updates the state of a tile based on the location of the cursor. This controlles the "hovered" state and highlights which ever tile the cursor is over
  (bind _index (Default|GetTileIndexUnderCursor (Variables|Default|Getgrid)))
  (if (!= _index (Variables|Default|Gethovered_tile))
    (Default|RemoveStatefromTile (Variables|Default|Getgrid) (Variables|Default|Gethovered_tile) "NewEnumerator1")
    (Variables|Default|Sethovered_tile _index)
    (Default|AddStatetoTile (Variables|Default|Getgrid) (Variables|Default|Gethovered_tile) "NewEnumerator1")
    (CallFunction|OnHoveredTileChange)))

(fn SetSelectedActions
  (params (Left%20Action :type BP%20Action%20Class%20Reference) (Right%20Action :type BP%20Action%20Class%20Reference))
  (Utilities|FlowControl|Sequence
    (:then_0
      (Utilities|IsValid (Variables|Default|GetselectedAction_LeftClick)
        (:Is%20Valid
          (Actor|DestroyActor (Variables|Default|GetselectedAction_LeftClick))
          (Variables|Default|SetselectedAction_LeftClick 0))
        (:Is%20Not%20Valid
          _))
      (if (Utilities|IsValidClass Left%20Action)
        (bind _returnvalue (Game|SpawnActorfromClass Left%20Action (Math|Transform|MakeTransform "0, 0, 0" "0, 0, 0" "1.000000,1.000000,1.000000") "AlwaysSpawn" 0 self 0))
        (Variables|Default|SetselectedAction_LeftClick _returnvalue)))
    (:then_1
      (Utilities|IsValid (Variables|Default|GetselectedAction_RightClick)
        (:Is%20Valid
          (Actor|DestroyActor (Variables|Default|GetselectedAction_RightClick))
          (Variables|Default|SetselectedAction_RightClick 0))
        (:Is%20Not%20Valid
          _))
      (if (Utilities|IsValidClass Right%20Action)
        (bind _returnvalue_2 (Game|SpawnActorfromClass Right%20Action (Math|Transform|MakeTransform "0, 0, 0" "0, 0, 0" "1.000000,1.000000,1.000000") "AlwaysSpawn" 0 self 0))
        (Variables|Default|SetselectedAction_RightClick _returnvalue_2)))
    (:then_2
      (Default|CallOnSelectedActionsChanged (Variables|Default|GetselectedAction_LeftClick) (Variables|Default|GetselectedAction_RightClick)))))