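; Tactical camera pawn that the player pans and zooms through axis inputs.
; Forward and strafe input shift a desired location along world X and Y, while zoom input adjusts a clamped desired spring arm length.
; Tick interpolates the actor location and spring arm length toward those targets for smooth camera motion, moving without collision sweep.
; Input steps are not scaled by delta time.
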(event EventTick
  (params (DeltaSeconds :type Float%20%28single-precision%29))
  ;[1 1 1] Uses interoplation to smooth out the zoom
  (Variables|/Script/Engine.SpringArmComponent|SetTargetArmLength (Variables|Default|GetSpringArm) (Math|Interpolation|FInterpTo (Variables|/Script/Engine.SpringArmComponent|GetTargetArmLength (Variables|Default|GetSpringArm)) (Variables|Default|Getzoom_desire) DeltaSeconds 2.0))
  ;[1 1 1] Handles controlling the camera location
  (Transformation|SetActorLocation (Math|Interpolation|VInterpTo (Transformation|GetActorLocation) (Variables|Default|Getlocation_desired) DeltaSeconds 5.0) false false))

(event EventBeginPlay
  (Variables|Default|Setlocation_desired (Transformation|GetActorLocation)))

(event Input|AxisEvents|InputAxisinput_axis_zoom
  (params (AxisValue :type Float%20%28single-precision%29))
  ;[1 1 1] Sets the zoom length
  (Variables|Default|Setzoom_desire (Math|Float|Clamp(Float) (+ (Variables|Default|Getzoom_desire) (* AxisValue 1e+02)) 1e+02 5e+03)))

(event Input|AxisEvents|InputAxisinput_axis_forward
  (params (AxisValue :type Float%20%28single-precision%29))
  (Variables|Default|Setlocation_desired (+ (Variables|Default|Getlocation_desired) (Math|Vector|MakeVector (* AxisValue 4e+01) 0.0 0.0))))

(event Input|AxisEvents|InputAxisinput_axis_strafe
  (params (AxisValue :type Float%20%28single-precision%29))
  (Variables|Default|Setlocation_desired (+ (Variables|Default|Getlocation_desired) (Math|Vector|MakeVector 0.0 (* AxisValue 2e+01) 0.0))))

(fn ConstructionScript)