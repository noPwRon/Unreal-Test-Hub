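; Grid pathfinding Blueprint that runs an A* search between two walkable tiles on square, hexagon or triangle grids.
; Shape-specific neighbour functions supply candidates, filtered by walkable type and height step, with optional diagonals for squares and triangles.
; FindPath expands the cheapest tile from a cost-sorted open list, recording previous tiles until it discovers the target.
; GeneratePath begins its back-trace at StartIndex rather than the target, so it adds no tiles.
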(event EventBeginPlay)

(event Collision|EventActorBeginOverlap
  (params (OtherActor :type Actor%20Object%20Reference)))

(event EventTick
  (params (DeltaSeconds :type Float%20%28single-precision%29)))

(fn ConstructionScript)

(fn GetValidTileNeighbours
  (params (index :type Int%20Point%20Structure) (include_diagonals :type Boolean))
  (LocalVariables|Setinput_data (.Value (Utilities|Map|Find (Variables|/Game/Blueprints/Core/Grid/BP_Grid.BP_Grid_C|GetGridTiles (Variables|Default|Getgrid)) index)))
  (bind _neighbours (Neighbours|GetNeighbourIndexes index include_diagonals))
  (for _array_element _neighbours
    (bind _output_get (LocalVariables|Setdata (.Value (Utilities|Map|Find (Variables|/Game/Blueprints/Core/Grid/BP_Grid.BP_Grid_C|GetGridTiles (Variables|Default|Getgrid)) _array_element))))
    (if (CallFunction|IsTileTypeWalkable (.type _output_get))
      (if (>= (.z (Variables|/Game/Blueprints/Core/Grid/BP_Grid.BP_Grid_C|GetGridTileSize (Variables|Default|Getgrid))) (Math|Float|Absolute(Float) (- (.z (.location (.transform (LocalVariables|Getdata)))) (.z (.location (.transform (LocalVariables|Getinput_data)))))))
        (Utilities|Array|Add (LocalVariables|GetRet) (Utilities|Struct|MakeS_pathfinding_data (.index (LocalVariables|Getdata)) 1 99999999 99999999 index)))))
  (return (LocalVariables|GetRet)))

(fn GetNeighbourIndexesforSquare
  (params (index :type Int%20Point%20Structure) (include_diagonals :type Boolean))
  (bind _returnvalue (+ index (Utilities|Struct|MakeIntPoint 1 0)))
  (bind _returnvalue_2 (+ index (Utilities|Struct|MakeIntPoint -1 0)))
  (bind _returnvalue_3 (+ index (Utilities|Struct|MakeIntPoint 0 1)))
  (bind _returnvalue_4 (+ index (Utilities|Struct|MakeIntPoint 0 -1)))
  (bind _array (Utilities|Array|MakeArray _returnvalue _returnvalue_2 _returnvalue_3 _returnvalue_4))
  (if include_diagonals
    (LocalVariables|SetRet _array)
    (Utilities|Array|AppendArray (LocalVariables|GetRet) (Utilities|Array|MakeArray (+ index (Utilities|Struct|MakeIntPoint 1 1)) (+ index (Utilities|Struct|MakeIntPoint -1 -1)) (+ index (Utilities|Struct|MakeIntPoint -1 1)) (+ index (Utilities|Struct|MakeIntPoint 1 -1))))
    (return (LocalVariables|GetRet))
    (else
      (return _array))))

(fn GetNeighbourIndexesforTriangle
  (params (index :type Int%20Point%20Structure) (include_diagonals :type Boolean))
  (LocalVariables|SetRet (Utilities|Array|MakeArray (+ index (Utilities|Struct|MakeIntPoint 0 -1)) (+ index (Utilities|Struct|MakeIntPoint 0 1))))
  (if (Utilities|EvenOddCheck index)
    ;[1 1 1] Find the neighbour tile based on the direction of the triangle
    (Utilities|Array|Add (LocalVariables|GetRet) (+ index (Utilities|Struct|MakeIntPoint -1 0)))
    (else
      (Utilities|Array|Add (LocalVariables|GetRet) (+ index (Utilities|Struct|MakeIntPoint 1 0)))))
  (if include_diagonals
    ;[1 1 1] Find the diagonal triangles depending on if the triangle is pointing up or down. Which is based on whether or not x and y are even or odd
    (if (Utilities|EvenOddCheck index)
      (Utilities|Array|AppendArray (LocalVariables|GetRet) (Utilities|Array|MakeArray (+ index (Utilities|Struct|MakeIntPoint 1 0)) (+ index (Utilities|Struct|MakeIntPoint -1 2)) (+ index (Utilities|Struct|MakeIntPoint -1 -2))))
      (else
        (Utilities|Array|AppendArray (LocalVariables|GetRet) (Utilities|Array|MakeArray (+ index (Utilities|Struct|MakeIntPoint -1 0)) (+ index (Utilities|Struct|MakeIntPoint 1 2)) (+ index (Utilities|Struct|MakeIntPoint 1 -2))))))
    (return (LocalVariables|GetRet))
    (else
      (for _array_element (LocalVariables|GetRet)
        (Development|PrintString (Utilities|String|ToString(Integer) _array_element))
        (return (LocalVariables|GetRet))))))

(fn GetNeighbourIndexesforHexagon
  (params (index :type Int%20Point%20Structure))
  (return (Utilities|Array|MakeArray (+ index (Utilities|Struct|MakeIntPoint -1 -1)) (+ index (Utilities|Struct|MakeIntPoint 1 -1)) (+ index (Utilities|Struct|MakeIntPoint 1 1)) (+ index (Utilities|Struct|MakeIntPoint 0 2)) (+ index (Utilities|Struct|MakeIntPoint 0 -2)) (+ index (Utilities|Struct|MakeIntPoint -1 1)))))

(fn EvenOddCheck
  (params (index :type Int%20Point%20Structure))
  (return (== (CallFunction|IsIntEven (.x index)) (CallFunction|IsIntEven (.y index)))))

(fn GetNeighbourIndexes
  (params (index :type Int%20Point%20Structure) (include_diagonals :type Boolean))
  (switch Utilities|FlowControl|Switch|SwitchonE_GridShape (Variables|/Game/Blueprints/Core/Grid/BP_Grid.BP_Grid_C|GetGridShape (Variables|Default|Getgrid))
    (:NewEnumerator1
      (return (Neighbours|GetNeighbourIndexesforSquare index include_diagonals)))
    (:NewEnumerator2
      (return (Neighbours|GetNeighbourIndexesforHexagon index)))
    (:NewEnumerator3
      (return (Neighbours|GetNeighbourIndexesforTriangle index include_diagonals)))))

(fn FindPath
  (params (start :type Int%20Point%20Structure) (target :type Int%20Point%20Structure) (Diagonals :type Boolean))
  (Variables|Default|SetStart_index start)
  (Variables|Default|SetTarget_index target)
  (Variables|Default|Setinclude_diagonals Diagonals)
  (Pathfinding|ClearGeneratedData)
  (bind _is_valid (Utilities|IsInputDataValid))
  (if _is_valid
    (Pathfinding|DiscoverTile (Utilities|Struct|MakeS_pathfinding_data (Variables|Default|GetStart_index) 1 0 (Pathfinding|GetMinCostBetweenTwoTiles (Variables|Default|GetStart_index) (Variables|Default|GetTarget_index) (Variables|Default|Getinclude_diagonals)) "(X=-999,Y=-999)"))
    (while (> (Utilities|Array|Length (Variables|Discovered_tiles|Getdiscovered_tile_indexes)) 0)
      (bind _found_target_tile (Pathfinding|AnalyzeNextDiscoveredTile))
      (if _found_target_tile
        (bind _path (Pathfinding|GeneratePath))
        (return _path)))
    (return (Utilities|Array|MakeArray))
    (else
      (return (Utilities|Array|MakeArray)))))

(fn IsInputDataValid
  ;[1 1 1] is the target tile the same tile you are standing on?
  (if (!= (Variables|Default|GetStart_index) (Variables|Default|GetTarget_index))
    ;[1 1 1] is the tile walkable
    (for _array_element (Utilities|Array|MakeArray (Variables|Default|GetStart_index) (Variables|Default|GetTarget_index))
      (if (not (Default|IsTileWalkable (Variables|Default|Getgrid) _array_element))
        (return false)))
    (return true)
    (else
      (return false))))

(fn DiscoverTile
  (params (tile_path_data :type S%20Pathfinding%20Data%20Structure))
  (Utilities|Map|Add (Variables|Default|Getpathfinding_data) (Utilities|Struct|BreakS_pathfinding_data tile_path_data) tile_path_data)
  (Pathfinding|InsertTileinDiscvoveredArray tile_path_data))

(fn GetMinCostBetweenTwoTiles
  (params (index%201 :type Int%20Point%20Structure) (index%202 :type Int%20Point%20Structure) (diagonals :type Boolean))
  (bind _returnvalue (- index%201 index%202))
  (bind _returnvalue_2 (- index%202 index%201))
  (if diagonals
    (return (Math|Float|Ceil (Math|Float|Sqrt (Math|Conversions|ToFloat(Integer) (+ (* (.x _returnvalue_2) (.x _returnvalue_2)) (* (.y _returnvalue_2) (.y _returnvalue_2)))))))
    (else
      (return (+ (Math|Integer|Absolute(Integer) (.x _returnvalue)) (Math|Integer|Absolute(Integer) (.y _returnvalue)))))))

(fn AnalyzeNextDiscoveredTile
  (bind _tile_path_data (Pathfinding|FindCheapestTilefromDiscoveredList))
  (Variables|DiscoveredTiles|Setcurrent_discovered_tile _tile_path_data)
  (bind _neighbours (Neighbours|GetValidTileNeighbours (.Index (Utilities|Struct|BreakS_pathfinding_data (Variables|DiscoveredTiles|Getcurrent_discovered_tile))) (Variables|Default|Getinclude_diagonals)))
  (Variables|AnalyzedTiles|Setcurrent_neighbours _neighbours)
  (while (> (Utilities|Array|Length (Variables|AnalyzedTiles|Getcurrent_neighbours)) 0)
    (bind _is_target_tile (Pathfinding|DiscoverNextNeighbour))
    (if _is_target_tile
      (return true)))
  (return false))

(fn GeneratePath
  (LocalVariables|SetCurrent (Variables|Default|GetStart_index))
  (while (!= (LocalVariables|GetCurrent) (Variables|Default|GetStart_index))
    (Utilities|Array|Add (LocalVariables|Getinverted_path) (LocalVariables|GetCurrent))
    (LocalVariables|SetCurrent (Utilities|Struct|BreakS_pathfinding_data (.Value (Utilities|Map|Find (Variables|Default|Getpathfinding_data) (LocalVariables|GetCurrent))))))
  (bind _arrayelement (Utilities|Array|ReverseforEachLoop (LocalVariables|Getinverted_path))
    (:LoopBody
      (Utilities|Array|Add (LocalVariables|GetRet) _arrayelement))
    (:Completed
      (return (LocalVariables|GetRet)))))

(fn FindCheapestTilefromDiscoveredList
  (LocalVariables|Settile_index (Utilities|Array|Get(acopy) (Variables|Discovered_tiles|Getdiscovered_tile_indexes)))
  (Utilities|Array|RemoveIndex (Variables|DiscoveredTiles|Getdiscovered_tile_sorting_costs))
  (Utilities|Array|RemoveIndex (Variables|Discovered_tiles|Getdiscovered_tile_indexes))
  (Utilities|Array|Add (Variables|AnalyzedTiles|Getanalyzed_tile_indexes) (LocalVariables|Gettile_index))
  (return (.Value (Utilities|Map|Find (Variables|Default|Getpathfinding_data) (LocalVariables|Gettile_index)))))

(fn DiscoverNextNeighbour
  (Variables|AnalyzedTiles|Setcurrent_neighbour (Utilities|Array|Get(acopy) (Variables|AnalyzedTiles|Getcurrent_neighbours)))
  (Utilities|Array|RemoveIndex (Variables|AnalyzedTiles|Getcurrent_neighbours))
  (if (not (Utilities|Array|ContainsItem (Variables|AnalyzedTiles|Getanalyzed_tile_indexes) (Utilities|Struct|BreakS_pathfinding_data (Variables|AnalyzedTiles|Getcurrent_neighbour)))) ; already analysed?
    (LocalVariables|Setcost_from_start (+ (Utilities|Struct|BreakS_pathfinding_data (Variables|DiscoveredTiles|Getcurrent_discovered_tile)) (Utilities|Struct|BreakS_pathfinding_data (Variables|AnalyzedTiles|Getcurrent_neighbour))))
    (bind _output_get (LocalVariables|Setindex_in_discovered (Utilities|Array|FindItem (Variables|Discovered_tiles|Getdiscovered_tile_indexes) (.Index (Utilities|Struct|BreakS_pathfinding_data (Variables|AnalyzedTiles|Getcurrent_neighbour)))))) ; find which index it is in discovered
    (if (== _output_get -1) ; new neighbour?
      _
      (else
        (bind _output_get_2 (Variables|AnalyzedTiles|Setcurrent_neighbour (.Value (Utilities|Map|Find (Variables|Default|Getpathfinding_data) (Utilities|Struct|BreakS_pathfinding_data (Variables|AnalyzedTiles|Getcurrent_neighbour))))))
        (if (< (LocalVariables|Getcost_from_start) (.Cost_to_start (Utilities|Struct|BreakS_pathfinding_data _output_get_2))) ; Found better path?
          (Utilities|Array|RemoveIndex (Variables|Discovered_tiles|Getdiscovered_tile_indexes) (LocalVariables|Getindex_in_discovered))
          (Utilities|Array|RemoveIndex (Variables|DiscoveredTiles|Getdiscovered_tile_sorting_costs) (LocalVariables|Getindex_in_discovered))
          (else
            (return false)))))
    (Pathfinding|DiscoverTile (Utilities|Struct|MakeS_pathfinding_data (.Index (Utilities|Struct|BreakS_pathfinding_data (Variables|AnalyzedTiles|Getcurrent_neighbour))) (.Cost_to_enter_tile (Utilities|Struct|BreakS_pathfinding_data (Variables|AnalyzedTiles|Getcurrent_neighbour))) (LocalVariables|Getcost_from_start) (Pathfinding|GetMinCostBetweenTwoTiles (Utilities|Struct|BreakS_pathfinding_data (Variables|AnalyzedTiles|Getcurrent_neighbour)) (Variables|Default|GetTarget_index) (Variables|Default|Getinclude_diagonals)) (Utilities|Struct|BreakS_pathfinding_data (Variables|DiscoveredTiles|Getcurrent_discovered_tile))))
    (if (Class|KismetMathLibrary|EqualIntPointIntPoint (.Index (Utilities|Struct|BreakS_pathfinding_data (Variables|AnalyzedTiles|Getcurrent_neighbour))) (Variables|Default|GetTarget_index))
      (return true)
      (else
        (return false)))
    (else
      (return false))))

(fn InsertTileinDiscvoveredArray
  (params (tile_path_data :type S%20Pathfinding%20Data%20Structure))
  (bind (_cost_to_start _min_cost_to_target) (Utilities|Struct|BreakS_pathfinding_data tile_path_data))
  (bind _discovered_tile_sorting_costs (Variables|DiscoveredTiles|Getdiscovered_tile_sorting_costs))
  (LocalVariables|Setsorting_cost (+ _cost_to_start _min_cost_to_target))
  (if (== (Utilities|Array|Length (Variables|DiscoveredTiles|Getdiscovered_tile_sorting_costs)) 0)
    ;[1 1 1] init cost array
    (Utilities|Array|Add (Variables|DiscoveredTiles|Getdiscovered_tile_sorting_costs) (LocalVariables|Getsorting_cost) :!label _label)
    (Utilities|Array|Add (Variables|Discovered_tiles|Getdiscovered_tile_indexes) (Utilities|Struct|BreakS_pathfinding_data tile_path_data))
    (elif (>= (LocalVariables|Getsorting_cost) (Utilities|Array|Get(acopy) _discovered_tile_sorting_costs (Utilities|Array|LastIndex _discovered_tile_sorting_costs)))
      (goto _label)
      (else
        (bind (_array_element _array_index) (Utilities|Array|ForEachLoopwithBreak (Variables|DiscoveredTiles|Getdiscovered_tile_sorting_costs) :!label _label_2)
          (:LoopBody
            (if (>= _array_element (LocalVariables|Getsorting_cost))
              (Utilities|Array|Insert (Variables|DiscoveredTiles|Getdiscovered_tile_sorting_costs) (LocalVariables|Getsorting_cost) _array_index)
              (Utilities|Array|Insert (Variables|Discovered_tiles|Getdiscovered_tile_indexes) (Utilities|Struct|BreakS_pathfinding_data tile_path_data) _array_index)
              (goto _label_2 Break))))))))

(fn ClearGeneratedData
  (Utilities|Map|Clear (Variables|Default|Getpathfinding_data))
  (Utilities|Array|Clear (Variables|DiscoveredTiles|Getdiscovered_tile_sorting_costs))
  (Utilities|Array|Clear (Variables|Discovered_tiles|Getdiscovered_tile_indexes))
  (Utilities|Array|Clear (Variables|AnalyzedTiles|Getanalyzed_tile_indexes)))