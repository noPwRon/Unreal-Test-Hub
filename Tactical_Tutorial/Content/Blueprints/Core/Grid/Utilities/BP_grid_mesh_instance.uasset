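; Grid utility actor that draws one mesh at many grid indices through a single InstancedStaticMesh component.
; An init function sets the mesh, material, "Colour" parameter and collision.
; InstanceIndexes mirrors instance order, mapping each caller-supplied index to its instance for removal, and adding at an existing index replaces that instance.
; Instances use local-space transforms, and actor tick is disabled at BeginPlay.
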(event EventBeginPlay
  (Actor|Tick|SetActorTickEnabled false))

(event Collision|EventActorBeginOverlap
  (params (OtherActor :type Actor%20Object%20Reference)))

(event EventTick
  (params (DeltaSeconds :type Float%20%28single-precision%29)))

(fn ConstructionScript)

(fn AddInstance
  (params (index :type Int%20Point%20Structure%20%28by%20ref%29) (Transform :type Transform%20%28by%20ref%29))
  (CallFunction|RemoveInstance index)
  (Components|InstancedStaticMesh|AddInstance (Variables|Default|GetInstancedStaticMesh) Transform false)
  (Utilities|Array|Add (Variables|Default|Getinstance_indexes) index))

(fn RemoveInstance
  (params (index :type Int%20Point%20Structure%20%28by%20ref%29))
  (bind _instance_indexes (Variables|Default|Getinstance_indexes))
  (if (Utilities|Array|ContainsItem _instance_indexes index)
    (Class|InstancedStaticMeshComponent|RemoveInstance (Variables|Default|GetInstancedStaticMesh) (Utilities|Array|FindItem _instance_indexes index))
    (Utilities|Array|RemoveItem (Variables|Default|Getinstance_indexes) index)))

(fn ClearInstances
  (Components|InstancedStaticMesh|ClearInstances (Variables|Default|GetInstancedStaticMesh))
  (Utilities|Array|Clear (Variables|Default|Getinstance_indexes)))

(fn InitGridMeshInstance
  (params (Mesh :type Static%20Mesh%20Object%20Reference) (Material :type Material%20Interface%20Object%20Reference) (Colour :type Linear%20Color%20Structure) (Collision :type ECollisionEnabled%20Enum :default "NoCollision"))
  (bind _instancedstaticmesh (Variables|Default|GetInstancedStaticMesh))
  (Components|StaticMesh|SetStaticMesh _instancedstaticmesh Mesh)
  (Rendering|Material|SetMaterial _instancedstaticmesh 0 Material)
  (Rendering|Material|SetVectorParameterValueonMaterials _instancedstaticmesh "Colour" (Math|Conversions|ToVector(LinearColor) Colour))
  (Collision|SetCollisionEnabled _instancedstaticmesh Collision))