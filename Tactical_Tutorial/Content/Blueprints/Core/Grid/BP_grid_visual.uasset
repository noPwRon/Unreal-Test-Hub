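; BP_grid_visual is the actor that displays a tile grid, drawing tiles through a BP_grid_mesh_instance child actor.
; On init it takes the flat mesh and border material from the grid's current shape data, centers itself at world origin and applies a ground offset in Z.
; Tile updates remove the instance by index and re-add it only for walkable tile types.
; Destroying the visual clears all instances, and actor tick is disabled.
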(event EventBeginPlay
  (Actor|Tick|SetActorTickEnabled false))

(event Collision|EventActorBeginOverlap
  (params (OtherActor :type Actor%20Object%20Reference)))

(event EventTick
  (params (DeltaSeconds :type Float%20%28single-precision%29)))

(fn ConstructionScript)

(fn InitGridVisual
  (params (grid :type BP%20Grid%20Object%20Reference))
  (Variables|Default|SetGrid grid)
  (Variables|Default|Setgrid_mesh_inst (.AsBP%20Grid%20Mesh%20Instance (Utilities|Casting|CastToBP_grid_mesh_instance (Variables|/Script/Engine.ChildActorComponent|GetChildActor (Variables|Default|GetChildActor_grid_mesh_inst)))))
  (Default|InitGridMeshInstance :self (Variables|Default|Getgrid_mesh_inst) :Mesh (.flat_mesh (Utilities|Struct|Breaks_grid_shape_data (Default|GetCurrentShapeData (Variables|Default|GetGrid)))) :Material (.flat_border_material (Utilities|Struct|Breaks_grid_shape_data (Default|GetCurrentShapeData (Variables|Default|GetGrid)))) :Collision "QueryOnly")
  (Transformation|SetActorLocation "0, 0, 0" false false) ; Center grid in world
  (CallFunction|SetOffsetfromGround (Variables|Default|GetOffset_from_ground)))

(fn SetOffsetfromGround
  (params (offset :type Float%20%28double-precision%29))
  (bind _returnvalue (Transformation|GetActorLocation))
  (Variables|Default|SetOffset_from_ground offset)
  (Transformation|SetActorLocation (Math|Vector|MakeVector (.x _returnvalue) (.y _returnvalue) (Variables|Default|GetOffset_from_ground)) false false))

(fn DestoryGridVisual
  (bind _grid_mesh_inst (Variables|Default|Getgrid_mesh_inst))
  (Utilities|IsValid _grid_mesh_inst
    (:Is%20Valid
      (Default|ClearInstances _grid_mesh_inst))))

(fn UpdateTileVisual
  (params (data :type S%20Tile%20Data%20Structure))
  (Default|RemoveInstance (Variables|Default|Getgrid_mesh_inst) (.index data))
  (if (CallFunction|IsTileTypeWalkable (.type data))
    (Default|AddInstance (Variables|Default|Getgrid_mesh_inst) (.index data) (.transform data))))