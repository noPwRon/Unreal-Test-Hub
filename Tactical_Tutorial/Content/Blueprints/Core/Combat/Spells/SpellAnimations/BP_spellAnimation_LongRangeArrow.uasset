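; Spell animation actor that visually fires a long-range arrow from an origin tile to a target tile.
; On play it moves to the origin tile and faces the target using the tile indices.
; A timeline lerps it to the target with a height offset while driving the arrow's rotation and scale.
; It reports the tile hit once partway through the timeline and completes the animation when finished.
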(event EventBeginPlay
  (|CallParentFunction) ; This node is disabled and will not be called.\nDrag off pins to build functionality.
)

(event Collision|EventActorBeginOverlap
  (params (OtherActor :type Actor%20Object%20Reference)))

(event EventTick
  (params (DeltaSeconds :type Float%20%28single-precision%29)))

(event EventEventPlaySpellAnimation
  (bind _anim_rotationscalelocation (Variables|Default|GetAnim_RotationScaleLocation))
  ;[0 0 0] Figure out where the target is and look at it
  (Transformation|SetActorLocationAndRotation (.location (CallFunction|GetTileTransform (Variables|Default|GetoriginIndex))) (Math|Rotator|FindLookatRotation (Math|Conversions|ToVector(Vector2D) (Math|Conversions|ToVector2D(IntPoint) (Variables|Default|GetoriginIndex))) (Math|Conversions|ToVector(Vector2D) (Math|Conversions|ToVector2D(IntPoint) (Variables|Default|GettargetIndex)))))
  ;[0 0 0] To do, make this look pretty with the animation
  (bind (_direction _location_alpha _location_z _rotation_x _scale _rotation_y) (Timeline|Timeline_LongRangeArrow PlayFromStart)
    (:Update
      (Transformation|SetActorLocation (+ (Math|Vector|Lerp(Vector) (.location (CallFunction|GetTileTransform (Variables|Default|GetoriginIndex))) (.location (CallFunction|GetTileTransform (Variables|Default|GettargetIndex))) _location_alpha) (Math|Vector|MakeVector 0.0 0.0 _location_z)) false false)
      (Transformation|SetRelativeRotation _anim_rotationscalelocation (Math|Rotator|MakeRotator _rotation_x _rotation_y 0.0) false false)
      (Transformation|SetRelativeScale3D _anim_rotationscalelocation (Math|Conversions|ToVector(Float) _scale))
      (if (> (Components|Timeline|GetPlaybackPosition (Variables|Default|GetTimeline_LongRangeArrow)) 0.5)
        (Utilities|FlowControl|DoOnce false
          (:Completed
            (Default|CallOnSpellAnimationHitTile self (Variables|Default|GettargetIndex))))))
    (:Finished
      (CallFunction|EventCompleteSpellAnimation))))

(fn ConstructionScript
  (|CallParentFunction))