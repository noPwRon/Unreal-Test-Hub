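; Spell animation actor that flies a configurable mesh, material and colour from an origin transform to a target transform.
; On BeginPlay it applies the visuals and plays a rate-adjusted timeline that lerps location, rotation and scale, adding a fixed vertical lift plus an animated height-offset curve.
; When the timeline finishes, it broadcasts OnShapeAnimationCompleted and destroys itself after a short delay.
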(event EventBeginPlay
  (Components|StaticMesh|SetStaticMesh (Variables|Default|GetanimatedShape) (Variables|Default|Getmesh))
  (Rendering|Material|SetMaterial (Variables|Default|GetanimatedShape) 0 (Variables|Default|Getmaterial))
  (Rendering|Material|SetVectorParameterValueonMaterials (Variables|Default|GetanimatedShape) "Color" (Math|Conversions|ToVector(LinearColor) (Variables|Default|Getcolour)))
  (Components|Timeline|SetPlayRate (Variables|Default|GetTimeline_playAnimation) (Variables|Default|GetplayRate))
  (bind (_direction _transformalpha _heightoffset) (Timeline|Timeline_playAnimation PlayFromStart)
    (:Update
      (Transformation|SetActorTransform (Math|Transform|MakeTransform (+ (.location (Math|Transform|Lerp(Transform) (Variables|Default|GetoriginTransform) (Variables|Default|GettargetTransform) _transformalpha)) "0.000000,0.000000,100.000000" (Math|Vector|MakeVector 0.0 0.0 _heightoffset)) (.rotation (Math|Transform|Lerp(Transform) (Variables|Default|GetoriginTransform) (Variables|Default|GettargetTransform) _transformalpha)) (.scale (Math|Transform|Lerp(Transform) (Variables|Default|GetoriginTransform) (Variables|Default|GettargetTransform) _transformalpha)))))
    (:Finished
      (Default|CallOnShapeAnimationCompleted self)
      (Utilities|FlowControl|Delay 0.5)
      (Actor|DestroyActor))))

(fn ConstructionScript)