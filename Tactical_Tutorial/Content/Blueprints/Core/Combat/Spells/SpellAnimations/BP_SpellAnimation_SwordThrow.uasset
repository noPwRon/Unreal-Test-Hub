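; Spell animation actor for a thrown sword that travels from an origin tile to a target tile on the grid.
; On play it faces the target, then a SwordSwing timeline lerps its location between the tiles and drives rotation from a yaw-based lerp.
; Past 0.5 seconds of playback it reports the target tile hit once, and the timeline's end completes the animation.
; A to-do marks the visuals as unpolished.
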(event EventBeginPlay
  (|CallParentFunction) ; This node is disabled and will not be called.\nDrag off pins to build functionality.
)

(event Collision|EventActorBeginOverlap
  (params (OtherActor :type Actor%20Object%20Reference)))

(event EventTick
  (params (DeltaSeconds :type Float%20%28single-precision%29)))

(event EventEventPlaySpellAnimation
  (bind _originindex (Variables|Default|GetoriginIndex))
  (bind _transform (CallFunction|GetTileTransform _originindex))
  ;[0 0 0] Figure out where the target is and look at it
  (Transformation|SetActorLocationAndRotation (.location (CallFunction|GetTileTransform (Variables|Default|GetoriginIndex))) (Math|Rotator|FindLookatRotation (Math|Conversions|ToVector(Vector2D) (Math|Conversions|ToVector2D(IntPoint) (Variables|Default|GetoriginIndex))) (Math|Conversions|ToVector(Vector2D) (Math|Conversions|ToVector2D(IntPoint) (Variables|Default|GettargetIndex)))))
  ;[0 0 0] To do, make this look pretty with the animation
  (bind (_direction _relativelocation _relativerotation) (Timeline|SwordSwing PlayFromStart)
    (:Update
      (Transformation|SetActorLocationAndRotation (Math|Vector|Lerp(Vector) (.location (CallFunction|GetTileTransform (Variables|Default|GetoriginIndex))) (.location (CallFunction|GetTileTransform (Variables|Default|GettargetIndex))) _relativelocation) (Math|Conversions|RotationFromXVector (Math|Vector|Lerp(Vector) (Math|Vector|MakeVector 0.0 0.0 (.yaw (.rotation _transform))) (Math|Vector|MakeVector 0.0 0.0 (+ (.yaw (.rotation _transform)) 1.17e+03)) _relativerotation)))
      (if (> (Components|Timeline|GetPlaybackPosition (Variables|Default|GetSwordSwing)) 0.5)
        (Utilities|FlowControl|DoOnce false
          (:Completed
            (Default|CallOnSpellAnimationHitTile self (Variables|Default|GettargetIndex))))))
    (:Finished
      (CallFunction|EventCompleteSpellAnimation))))

(fn ConstructionScript
  (|CallParentFunction))