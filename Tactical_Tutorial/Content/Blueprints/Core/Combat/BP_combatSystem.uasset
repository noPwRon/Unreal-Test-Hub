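; BP_combatSystem manages the units in a grid-based combat and resolves spell casts.
; It keeps each unit's index, tile data and world position in sync, destroying units left on invalid tile types after grid or tile updates.
; Spell casts check pattern-based range, filtered by walkability and optional line-of-sight traces from four offset origins, then spawn the spell actor with the target or AOE tiles.
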(event EventBeginPlay
  (bind _grid (Variables|Default|GetGrid))
  (EventDispatchers|BindEventtoOnGridGenerated _grid (EventDispatchers|CreateEvent :!event OnGridGenerated))
  (EventDispatchers|BindEventtoOnTileDataUpdated _grid (EventDispatchers|CreateEvent :!event OnTileDataUpdated)))

(event Collision|EventActorBeginOverlap
  (params (OtherActor :type Actor%20Object%20Reference)))

(event EventTick
  (params (DeltaSeconds :type Float%20%28single-precision%29)))

(fn ConstructionScript)

(fn AddUnitinCombat
  (params (Unit :type BP%20Unit%20Object%20Reference) (Index :type Int%20Point%20Structure))
  ;[0 0 0] [EN] Add unit in combat list and then place it on the grid
  ; [FR] Ajouter l'unité dans la combat list et ensuite on la place sur la grille
  (Utilities|Array|Add (Variables|Default|GetUnitsInCombat) Unit)
  (Default|SetGrid Unit (Variables|Default|GetGrid))
  (Units|SetUnitIndexonGrid Unit Index false)
  (EventDispatchers|BindEventtoOnUnitReachedNewTile Unit (EventDispatchers|CreateEvent :!event OnUnitReachedNewTile)))

(fn RemoveUnitfromCombat
  (params (Unit :type BP%20Unit%20Object%20Reference) (DestroyActor :type Boolean))
  ;[0 0 0] [EN] Remove unit from list and from the grid. And also destroy it if requested
  ; [FR] Enlever l'unité de la liste et de la grille. Et ensuite la détruit si c'est ce qu'on veut
  (Utilities|Array|RemoveItem (Variables|Default|GetUnitsInCombat) Unit)
  (Units|SetUnitIndexonGrid Unit (Utilities|Struct|MakeIntPoint -999 -999) false)
  (if DestroyActor
    (Actor|DestroyActor Unit)))

(fn SetUnitIndexonGrid
  (params (Unit :type BP%20Unit%20Object%20Reference) (Index :type Int%20Point%20Structure) (Force :type Boolean))
  (bind _grid (Variables|Default|GetGrid))
  (bind _gridtiles (Variables|/Game/Blueprints/Core/Grid/BP_Grid.BP_Grid_C|GetGridTiles _grid))
  (bind (_value _returnvalue) (Utilities|Map|Find _gridtiles Index))
  (Utilities|FlowControl|Sequence
    (:then_0
      ;[0 0 0] [EN] If new index, we move the unit from the previous index to the new one
      ; [FR] Si l'index est différent, on déplace l'unité de l'index précédent vers le nouveau
      (if (or (!= (Variables|/Game/Blueprints/Core/Units/BP_Unit.BP_Unit_C|GetIndex Unit) Index) Force) ; Different Index?
        (Utilities|FlowControl|Sequence ; 0 = Remove from previous tile\n1 = Add to new tile
          (:then_0
            (bind _output_get (LocalVariables|SetPreviousTile (.Value (Utilities|Map|Find (Variables|/Game/Blueprints/Core/Grid/BP_Grid.BP_Grid_C|GetGridTiles (Variables|Default|GetGrid)) (Variables|/Game/Blueprints/Core/Units/BP_Unit.BP_Unit_C|GetIndex Unit)))))
            (if (== (Utilities|Struct|BreakS_TileData _output_get) Unit)
              (bind _structout (Utilities|Struct|SetmembersinS_TileData (LocalVariables|GetPreviousTile)))
              (Utilities|Map|Add (Variables|/Game/Blueprints/Core/Grid/BP_Grid.BP_Grid_C|GetGridTiles (Variables|Default|GetGrid)) (Utilities|Struct|BreakS_TileData _structout) _structout)))
          (:then_1
            (Default|SetGridIndex Unit Index)
            (if (!= Index (Utilities|Struct|MakeIntPoint -999 -999))
              (bind _structout_2 (Utilities|Struct|SetmembersinS_TileData (.Value (Utilities|Map|Find (Variables|/Game/Blueprints/Core/Grid/BP_Grid.BP_Grid_C|GetGridTiles (Variables|Default|GetGrid)) Index)) Unit))
              (Utilities|Map|Add (Variables|/Game/Blueprints/Core/Grid/BP_Grid.BP_Grid_C|GetGridTiles (Variables|Default|GetGrid)) (Utilities|Struct|BreakS_TileData _structout_2) _structout_2)))
          (:then_2
            (Default|CallOnUnitGridIndexChanged Unit)))))
    (:then_1
      ;[0 0 0] [EN] Then move the actor in the world
      ; [FR] Ensuite déplace l'acteur dans le monde
      (Transformation|SetActorLocation Unit (select _returnvalue (.location (Utilities|Struct|BreakS_TileData _value)) "-99999.000000,-99999.000000,-99999.000000") false false))))

(fn OnGridGenerated
  ;[0 0 0] [EN] When the grid is re-generated, we make sure the units are still on a valid index, otherwise we destroy them
  ; [FR] Quand la grille est regénérée, on fait sûr que les unités sont encore sur des cases valides, sinon on les détruits
  (bind _output_get (LocalVariables|SetCopyOfUnitsInCombat (Variables|Default|GetUnitsInCombat))) ; Becase we're modifying the real list
  (for _array_element _output_get
    (if (Utilities|Array|ContainsItem (.validtiletypes (.stats (Variables|/Game/Blueprints/Core/Units/BP_Unit.BP_Unit_C|GetUnitData _array_element))) (.type (.Value (Utilities|Map|Find (Variables|/Game/Blueprints/Core/Grid/BP_Grid.BP_Grid_C|GetGridTiles (Variables|Default|GetGrid)) (Variables|/Game/Blueprints/Core/Units/BP_Unit.BP_Unit_C|GetIndex _array_element)))))
      (Units|SetUnitIndexonGrid _array_element (Variables|/Game/Blueprints/Core/Units/BP_Unit.BP_Unit_C|GetIndex _array_element) true)
      (else
        (Units|RemoveUnitfromCombat _array_element true)))))

(fn OnTileDataUpdated
  (params (Index :type Int%20Point%20Structure))
  ;[0 0 0] [EN] When a tile is updated, we make sure the index is still valid for the unit, otherwise we destroy it
  ; [FR] Quand une case de la grille est mise a jour, on fait sûr que l'index est encore valide pour l'unité, sinon on la détruit
  (bind _output_get (LocalVariables|SetCopyOfUnitsInCombat (Variables|Default|GetUnitsInCombat))) ; Becase we're modifying the real list
  (bind _array_element (Utilities|Array|ForEachLoopwithBreak _output_get :!label _label)
    (:LoopBody
      (if (Class|KismetMathLibrary|EqualIntPointIntPoint Index (Variables|/Game/Blueprints/Core/Units/BP_Unit.BP_Unit_C|GetIndex _array_element))
        (if (Utilities|Array|ContainsItem (.validtiletypes (.stats (Variables|/Game/Blueprints/Core/Units/BP_Unit.BP_Unit_C|GetUnitData _array_element))) (.type (.Value (Utilities|Map|Find (Variables|/Game/Blueprints/Core/Grid/BP_Grid.BP_Grid_C|GetGridTiles (Variables|Default|GetGrid)) (Variables|/Game/Blueprints/Core/Units/BP_Unit.BP_Unit_C|GetIndex _array_element)))))
          (Units|SetUnitIndexonGrid _array_element (Variables|/Game/Blueprints/Core/Units/BP_Unit.BP_Unit_C|GetIndex _array_element) false)
          (goto _label Break)
          (else
            (Units|RemoveUnitfromCombat _array_element true)
            (goto _label Break)))))))

(fn OnUnitReachedNewTile
  (params (Unit :type BP%20Unit%20Object%20Reference) (Index :type Int%20Point%20Structure))
  ;[0 0 0] [EN] Unit reached a new tile, we have to update the index in the data. Later we might add some validations here
  ; [FR] L'unité a attein une nouvelle case, on doit mettre à jour son index dans le data. Plus tard, on va probablement ajouter des validations ici
  (Units|SetUnitIndexonGrid Unit Index false))

(fn CastSpell
  (params (spell :type E_Spell%20Enum :default "NewEnumerator0") (originIndex :type Int%20Point%20Structure) (targetIndex :type Int%20Point%20Structure))
  ;[0 0 0] Take in spell info
  (bind _spelldata (CallFunction|GetSpellDatafromSpell spell))
  (LocalVariables|SetData _spelldata)
  ;[0 0 0] Makes sure the spell is within range
  (bind _rangeindexes (CallFunction|GetSpellRange originIndex (.Cast (Utilities|Struct|BreakS_SpellData (LocalVariables|GetData)))))
  (if (Utilities|Array|ContainsItem _rangeindexes targetIndex)
    ;[0 0 0] Determine if the spell has AOE
    (if (Utilities|Enum|Equal(Enum) (.RangePattern (Utilities|Struct|BreakS_spellData_Cast (.CastAOE (Utilities|Struct|BreakS_SpellData (LocalVariables|GetData))))) "NewEnumerator0")
      ;[0 0 0] No AOE, just pass the target index
      (LocalVariables|SetattackedIndexes (Utilities|Array|MakeArray targetIndex))
      (else
        ;[0 0 0] Determine the AOE range and pass the indexs to the spell actor
        (bind _rangeindexes_2 (CallFunction|GetSpellRange targetIndex (.CastAOE (Utilities|Struct|BreakS_SpellData (LocalVariables|GetData)))))
        (LocalVariables|SetattackedIndexes _rangeindexes_2)))
    ;[0 0 0] cast the spell once all checks have been made.
    (Game|SpawnActorfromClass (Utilities|Struct|BreakS_SpellData_Assets (.Assets (Utilities|Struct|BreakS_SpellData (LocalVariables|GetData)))) (Math|Transform|MakeTransform "0, 0, 0" "0, 0, 0" "1.000000,1.000000,1.000000") "AlwaysSpawn" 0 (Variables|Default|GetGrid) originIndex (LocalVariables|GetattackedIndexes) 0)))

(fn GetSpellRange
  (params (originIndex :type Int%20Point%20Structure) (Cast :type S%20Spell%20Data%20Cast%20Structure))
  (bind (_rangepattern _rangeminmax _lineofsight) (Utilities|Struct|BreakS_spellData_Cast Cast))
  ;[0 0 0] Get the range and pattern
  (bind _rangeindexes (CallFunction|GetIndexesfromPatternandRange originIndex (Variables|/Game/Blueprints/Core/Grid/BP_Grid.BP_Grid_C|GetGridShape (Variables|Default|GetGrid)) _rangepattern _rangeminmax))
  ;[0 0 0] Remove invalid tiles
  (bind _validindexes (CallFunction|RemoveNotWalkableIndexes _rangeindexes))
  ;[0 0 0] Remove indexes if the spell is affected by line of sight
  (if (.requirelineofsight _lineofsight)
    (bind _validindexes_2 (CallFunction|RemoveIndexesWithoutLineOfSight originIndex _validindexes Cast))
    (return _validindexes_2)
    (else
      (return _validindexes))))

(fn HasLineOfSight
  (params (originIndex :type Int%20Point%20Structure) (targetIndex :type Int%20Point%20Structure) (Cast :type S%20Spell%20Data%20Cast%20Structure))
  (bind _grid (Variables|Default|GetGrid))
  (bind _grid_2 (Variables|Default|GetGrid))
  (bind _lineofsight (Utilities|Struct|BreakS_spellData_Cast Cast))
  (bind _lineofsight_2 (Utilities|Struct|BreakS_spellData_Cast Cast))
  (bind _gridtiles (Variables|/Game/Blueprints/Core/Grid/BP_Grid.BP_Grid_C|GetGridTiles _grid))
  (bind _gridtilesize (Variables|/Game/Blueprints/Core/Grid/BP_Grid.BP_Grid_C|GetGridTileSize _grid_2))
  (bind _returnvalue (Math|Vector|MakeVector 0.0 0.0 (.lineofsight_heightfromground _lineofsight)))
  (bind _returnvalue_2 (* _gridtilesize (.lineofsight_offsetfromcenter _lineofsight_2)))
  (LocalVariables|SetoriginTile (.Value (Utilities|Map|Find _gridtiles originIndex)))
  (LocalVariables|SettargetTile (.Value (Utilities|Map|Find _gridtiles targetIndex)))
  (LocalVariables|Setstart (+ (.location (Utilities|Struct|BreakS_TileData (LocalVariables|GetoriginTile))) _returnvalue))
  (LocalVariables|Setend (+ _returnvalue (.location (Utilities|Struct|BreakS_TileData (LocalVariables|GettargetTile)))))
  (for _array_element (Utilities|Array|MakeArray (Math|Vector2D|MakeVector2D (.x _returnvalue_2) 0.0) (Math|Vector2D|MakeVector2D (- 0.0 (.x _returnvalue_2)) 0.0) (Math|Vector2D|MakeVector2D 0.0 (.y _returnvalue_2)) (Math|Vector2D|MakeVector2D 0.0 (- 0.0 (.y _returnvalue_2))))
    (bind _returnvalue_3 (Collision|LineTraceByChannel (+ (LocalVariables|Getstart) (Math|Conversions|ToVector(Vector2D) _array_element)) (LocalVariables|Getend) "TraceTypeQuery5" false (Utilities|Array|MakeArray (Utilities|Struct|BreakS_TileData (LocalVariables|GetoriginTile)) (Utilities|Struct|BreakS_TileData (LocalVariables|GettargetTile))) (select (.lineofsight_drawdebugline (Utilities|Struct|BreakS_spellData_Cast Cast)) "ForDuration" "None")))
    (if (not _returnvalue_3)
      (return true)))
  (return false))

(fn RemoveIndexesWithoutLineOfSight
  (params (originIndex :type Int%20Point%20Structure) (indexes :type Array%20of%20Int%20Point%20Structures) (Cast :type S%20Spell%20Data%20Cast%20Structure))
  (for _array_element indexes
    (if (CallFunction|HasLineOfSight originIndex _array_element Cast)
      (Utilities|Array|Add (LocalVariables|GetRet) _array_element)))
  (return (LocalVariables|GetRet)))

(fn RemoveNotWalkableIndexes
  (params (indexes :type Array%20of%20Int%20Point%20Structures))
  (for _array_element indexes
    (if (Default|IsTileWalkable (Variables|Default|GetGrid) _array_element)
      (Utilities|Array|Add (LocalVariables|GetRet) _array_element)))
  (return (LocalVariables|GetRet)))