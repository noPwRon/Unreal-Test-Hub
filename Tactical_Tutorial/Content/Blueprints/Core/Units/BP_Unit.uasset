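; Grid-based unit actor whose mesh and anim Blueprint are set from its unit type in the construction script.
; It walks a given path tile by tile, using a timeline to interpolate location and rotation, hop between differing heights and fire movement events.
; A line-of-sight collision mesh follows the grid's tile shape, size and rotation.
; Hover and selection states tint the mesh through a material color parameter.
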(event Custom|ContinueToFollowPath
  (bind _timeline_unitmovement (Variables|Default|GetTimeline_UnitMovement))
  (bind _grid (Variables|Default|GetGrid))
  (bind _currentpathtofollow (Variables|UnitMovement|GetCurrentPathToFollow))
  (bind _output (Utilities|Array|Get(acopy) _currentpathtofollow))
  (bind _gridtiles (Variables|/Game/Blueprints/Core/Grid/BP_Grid.BP_Grid_C|GetGridTiles _grid))
  (bind _value (Utilities|Map|Find _gridtiles _output))
  (bind _transform (Utilities|Struct|BreakS_TileData _value))
  ;[0 0 0] [EN] Not done walking? Continue
  ; [FR] Pas terminé de marcher? Continue
  (if (> (Utilities|Array|Length (Variables|UnitMovement|GetCurrentPathToFollow)) 0)
    (CallFunction|SetAnimationState "NewEnumerator1")
    ;[0 0 0] [EN] Set the current tile and next tile for the interpolation
    ; [FR] Set la case courante et la prochaine case pour l'interpolation
    (Variables|UnitMovement|SetPreviousTransform (Transformation|GetActorTransform))
    (Variables|UnitMovement|SetNextTransform (Math|Transform|MakeTransform (.location _transform) (Math|Rotator|MakeRotator 0.0 0.0 (.yaw (Math|Rotator|FindLookatRotation (.location (Variables|UnitMovement|GetPreviousTransform)) (.location _transform)))) "1.000000,1.000000,1.000000"))
    ;[0 0 0] [EN] Apply desired speed to the timeline
    ; [FR] Appliquer la vitesse voulue à la timeline
    (Components|Timeline|SetPlayRate _timeline_unitmovement (/ (Components|Timeline|GetTimelineLength _timeline_unitmovement) (Variables|UnitMovement|GetMoveDurationPerTile)))
    ;[0 0 0] [EN] Move the unit based on the timeline: Interpolate position to next tile. Look at next tile. If there's a height difference, add a little jump on the location.
    ; [FR] Déplace l'unité basé sur la timeline: Interpole la position vers la prochaine case. Regarde la prochaine case. S'il y a une différence de hauteur, ajoute un petit saut à la location.
    (bind (_direction _locationalpha _rotationalpha _jump) (Timeline|Timeline_UnitMovement PlayFromStart)
      (:Update
        (Transformation|SetActorLocationAndRotation (+ (Math|Vector|Lerp(Vector) (.location (Variables|UnitMovement|GetPreviousTransform)) (.location (Variables|UnitMovement|GetNextTransform)) _locationalpha) (Math|Vector|MakeVector 0.0 0.0 (select (Math|Float|NearlyEqual(Float) (.z (.location (Variables|UnitMovement|GetPreviousTransform))) (.z (.location (Variables|UnitMovement|GetNextTransform))) 5.0) 0.0 _jump))) (Math|Rotator|Lerp(Rotator) (.rotation (Variables|UnitMovement|GetPreviousTransform)) (.rotation (Variables|UnitMovement|GetNextTransform)) _rotationalpha true)))
      (:Finished
        ;[0 0 0] [EN] Next tile reached, remove it from the path and do the next loop
        ; [FR] Arrivé sur la case suivante. Enlève là du path et ensuite exécute la prochaine loop
        (Default|CallOnUnitReachedNewTile self (Utilities|Array|Get(acopy) (Variables|UnitMovement|GetCurrentPathToFollow)))
        (Utilities|Array|RemoveIndex (Variables|UnitMovement|GetCurrentPathToFollow))
        (CallFunction|ContinuetoFollowPath)))
    (else
      ;[0 0 0] [EN] End of the movement
      ; [FR] Fin du mouvement
      (CallFunction|SetAnimationState "NewEnumerator0")
      (Default|CallOnUnitFinishedWalking self))))

(event Custom|Event_FollowPath
  (params (Path :type Array%20of%20Int%20Point%20Structures))
  ;[0 0 0] [EN] Beginning of the movement
  ; [FR] Début du mouvement
  (if (> (Utilities|Array|Length Path) 0)
    (Variables|UnitMovement|SetCurrentPathToFollow Path)
    (Default|CallOnUnitStartedWalking self)
    (CallFunction|ContinuetoFollowPath)))

(event EventBeginPlay
  (CallFunction|SetAnimationState "NewEnumerator0"))

(fn ConstructionScript
  (bind _unitdata (CallFunction|GetDefaultUnitDatafromUnitType (Variables|Default|GetUnitType)))
  (CallFunction|SetUnitData _unitdata))

(fn UpdateVisualifHoveredorSelected
  (Rendering|Material|SetVectorParameterValueonMaterials (Variables|Default|GetSkeletalMesh) "ColorMultiply" (Math|Conversions|ToVector(LinearColor) (* (* (select (Variables|Hovered&Selected|GetIsSelected) "(R=0.176490,G=0.523803,B=1.000000,A=1.000000)" "(R=1.000000,G=1.000000,B=1.000000,A=1.000000)") (select (Variables|Hovered&Selected|GetIsHovered) 2.5 1.0)) (select (Variables|Hovered&Selected|GetIsSelected) 2.5 1.0)))))

(fn SetIsHovered
  (params (Hovered :type Boolean))
  (Variables|Hovered&Selected|SetIsHovered Hovered)
  (Hovered&Selected|UpdateVisualifHoveredorSelected))

(fn SetIsSelected
  (params (Selected :type Boolean))
  (Variables|Hovered&Selected|SetIsSelected Selected)
  (Hovered&Selected|UpdateVisualifHoveredorSelected))

(fn SetUnitData
  (params (Data :type S%20Unit%20Data%20Structure%20%28by%20ref%29))
  (bind _skeletalmesh (Variables|Default|GetSkeletalMesh))
  (bind _output_get (Variables|Default|SetUnitData Data))
  (Components|SkinnedMesh|SetSkinnedAssetandUpdate _skeletalmesh (.Mesh (Utilities|Struct|BreakS_UnitData_Assets (.Assets (Utilities|Struct|BreakS_UnitData _output_get)))) true)
  (Class|SkeletalMeshComponent|SetAnimClass _skeletalmesh (.AnimBp (Utilities|Struct|BreakS_UnitData_Assets (.Assets (Utilities|Struct|BreakS_UnitData _output_get))))))

(fn SetAnimationState
  (params (State :type E_UnitAnimationState%20Enum :default "NewEnumerator0"))
  (Class|BPIUnitAnimation|SetUnitAnimationState(Message) (Components|SkeletalMesh|GetAnimInstance (Variables|Default|GetSkeletalMesh)) State))

(fn SetGrid
  (params (Grid :type BP%20Grid%20Object%20Reference))
  (bind _collision_lineofsight (Variables|Default|GetCollision_lineOfSight))
  (Variables|Default|SetGrid Grid)
  (Components|StaticMesh|SetStaticMesh _collision_lineofsight (.Mesh (Utilities|Struct|BreakS_GridShapeData (Default|GetCurrentShapeData (Variables|Default|GetGrid)))))
  (Transformation|SetAbsolute _collision_lineofsight false true true)
  (Transformation|SetWorldScale3D _collision_lineofsight (Math|Vector|MakeVector (.x (/ (Variables|/Game/Blueprints/Core/Grid/BP_Grid.BP_Grid_C|GetGridTileSize (Variables|Default|GetGrid)) (.MeshSize (Utilities|Struct|BreakS_GridShapeData (Default|GetCurrentShapeData (Variables|Default|GetGrid)))))) (.y (/ (Variables|/Game/Blueprints/Core/Grid/BP_Grid.BP_Grid_C|GetGridTileSize (Variables|Default|GetGrid)) (.MeshSize (Utilities|Struct|BreakS_GridShapeData (Default|GetCurrentShapeData (Variables|Default|GetGrid)))))) (.z (Transformation|GetWorldScale (Variables|Default|GetCollision_lineOfSight)))))
  (Transformation|SetWorldRotation _collision_lineofsight (Default|GetTileRotationfromGridIndex (Variables|Default|GetGrid) (Variables|Default|GetIndex)) false false))

(fn SetGridIndex
  (params (index :type Int%20Point%20Structure))
  (Variables|Default|SetIndex index)
  (Transformation|SetWorldRotation (Variables|Default|GetCollision_lineOfSight) (Default|GetTileRotationfromGridIndex (Variables|Default|GetGrid) (Variables|Default|GetIndex)) false false))