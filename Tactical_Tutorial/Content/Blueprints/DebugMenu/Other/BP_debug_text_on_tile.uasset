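; Debug actor that labels each walkable tile of BP_Grid with its X,Y index using spawned text render actors.
; On BeginPlay it finds the grid and binds to its tile-updated and grid-destroyed events.
; Texts are cached in a map by index, created on demand without tick or collision, and destroyed when the tile is missing or unwalkable.
; A toggle rebuilds or clears all labels.
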(event EventBeginPlay
  (bind _returnvalue (Actor|GetActorOfClass "/Game/Blueprints/Core/Grid/BP_Grid.BP_Grid_C"))
  (bind _output_get (Variables|Default|Setgrid _returnvalue))
  (EventDispatchers|BindEventtoOnTileDataUpdated _output_get (EventDispatchers|CreateEvent :!event UpdateTextonTile))
  (EventDispatchers|BindEventtoOnGridDestroyed _output_get (EventDispatchers|CreateEvent :!event ClearAllTextActors)))

(event Collision|EventActorBeginOverlap
  (params (OtherActor :type Actor%20Object%20Reference)))

(event EventTick
  (params (DeltaSeconds :type Float%20%28single-precision%29)))

(fn ConstructionScript)

(fn GetTextActor
  (params (index :type Int%20Point%20Structure))
  (bind _output_get (LocalVariables|Setactor (.Value (Utilities|Map|Find (Variables|Default|Getspawned_texts) index))))
  (Utilities|IsValid _output_get
    (:Is%20Valid
      (return (LocalVariables|Getactor)))
    (:Is%20Not%20Valid
      (bind _returnvalue (Game|SpawnActorfromClass "/Script/Engine.TextRenderActor" (Math|Transform|MakeTransform "0, 0, 0" "0, 0, 0" "1.000000,1.000000,1.000000") "AlwaysSpawn" 0 0))
      (LocalVariables|Setactor _returnvalue)
      (Utilities|Map|Add (Variables|Default|Getspawned_texts) index (LocalVariables|Getactor))
      ;[1 1 1] make sure collisions aren't enabled because that would be useless for debug text
      (Actor|Tick|SetActorTickEnabled (LocalVariables|Getactor))
      (Collision|SetActorEnableCollision (LocalVariables|Getactor) false)
      ;[1 1 1] set the alignment of the text
      (Rendering|Components|TextRender|SetHorizontalAlignment (Variables|/Script/Engine.TextRenderActor|GetTextRender (LocalVariables|Getactor)) "EHTA_Center")
      (Class|TextRenderComponent|SetVerticalAlignment (Variables|/Script/Engine.TextRenderActor|GetTextRender (LocalVariables|Getactor)) "EVRTA_TextCenter")
      (return (LocalVariables|Getactor)))))

(fn DestroyTextActor
  (params (index :type Int%20Point%20Structure))
  (bind _output_get (LocalVariables|Setactor (.Value (Utilities|Map|Find (Variables|Default|Getspawned_texts) index))))
  (Utilities|IsValid _output_get
    (:Is%20Valid
      (Actor|DestroyActor _output_get)
      (Utilities|Map|Remove (Variables|Default|Getspawned_texts) index))))

(fn ClearAllTextActors
  (bind _spawned_texts (Variables|Default|Getspawned_texts))
  (bind _values (Utilities|Map|Values _spawned_texts))
  (for _array_element _values
    (Actor|DestroyActor _array_element))
  (Utilities|Map|Clear _spawned_texts))

(fn UpdateTextonTile
  (params (index :type Int%20Point%20Structure))
  (bind _grid (Variables|Default|Getgrid))
  (bind _gridtiles (Variables|/Game/Blueprints/Core/Grid/BP_Grid.BP_Grid_C|GetGridTiles _grid))
  (bind (_value _returnvalue) (Utilities|Map|Find _gridtiles index))
  (if (Variables|Default|Getshow_tile_indexes)
    (if _returnvalue
      (LocalVariables|Setdata _value)
      (if (CallFunction|IsTileTypeWalkable (.type (LocalVariables|Getdata)))
        (bind _text_render_actor (CallFunction|GetTextActor index))
        (LocalVariables|Settext_actor _text_render_actor)
        (LocalVariables|Settext (Utilities|String|Append (Utilities|String|ToString(Integer) (.x index)) "," (Utilities|String|ToString(Integer) (.y index))))
        (Rendering|Components|TextRender|SetText (Variables|/Script/Engine.TextRenderActor|GetTextRender (LocalVariables|Gettext_actor)) (Utilities|Text|ToText(String) (LocalVariables|Gettext)))
        (Transformation|SetActorTransform (LocalVariables|Gettext_actor) (Math|Transform|MakeTransform (+ (.location (.transform (LocalVariables|Getdata))) "0.000000,0.000000,1.000000") "90.000000,180.000000,0.000000" "2.000000,2.000000,2.000000"))
        (else
          (CallFunction|DestroyTextActor index :!label _label)))
      (else
        (goto _label)))))

(fn SetShowTileIndexes
  (params (show_tile_indexes :type Boolean))
  (bind _output_get (Variables|Default|Setshow_tile_indexes show_tile_indexes))
  (if _output_get
    (bind _keys (Utilities|Map|Keys (Variables|/Game/Blueprints/Core/Grid/BP_Grid.BP_Grid_C|GetGridTiles (Variables|Default|Getgrid))))
    (for _array_element _keys
      (CallFunction|UpdateTextonTile _array_element))
    (else
      (CallFunction|ClearAllTextActors))))