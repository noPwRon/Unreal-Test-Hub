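; Ranger AI class for combat units that switches movement logic and spell scoring when the unit drops below half health.
; Each turn it refreshes the health flag, then keeps the top-scoring cast, summing impact on units hit, itself included.
; Travel distance to the casting cell adds to the score when healthy and subtracts when hurt.
; A post-decision override sketches a self-targeted fallback such as a dash, while other overrides just call the parent.
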(event EventBeginPlay
  (|CallParentFunction) ; This node is disabled and will not be called.\nDrag off pins to build functionality.
)

(event Collision|EventActorBeginOverlap
  (params (OtherActor :type Actor%20Object%20Reference)))

(event EventTick
  (params (DeltaSeconds :type Float%20%28single-precision%29)))

(event EventDecideWhichSpelltoCastDone
  (bind _unit (Variables|Default|Getunit))
  (bind _index (Variables|/Game/Blueprints/Core/Units/BP_Unit.BP_Unit_C|GetIndex _unit))
  ;[0 0 0] An example of overriding the chosen spell. This assumes that there were some reasons for why the spell wan't chosen in the first place. (This could be where a dash action is added if all other options dont work)
  (Utilities|FlowControl|Sequence
    (:then_0
      (if (Utilities|Struct|BreakS_unitAiSpellCastingData (Variables|Default|GetaiSpellCasting)) ; If no available spells then we will get the "Dash" function
        (bind _spelldata (CallFunction|GetSpellDatafromSpell "NewEnumerator0"))
        (bind _cancast (Default|CanCastSpell _unit _spelldata))
        (if _cancast
          (Variables|Default|SetaiSpellCasting (Utilities|Struct|MakeS_unitAiSpellCastingData _cancast "NewEnumerator0" _index _index)))))
    (:then_1
      (|CallParentFunction))))

(fn ConstructionScript
  (|CallParentFunction))

(fn AiPlayTurn
  (bind _unit (Variables|Default|Getunit))
  (Variables|Default|SethalfHealth (< (/ (Default|GetCurrentHp _unit) (Default|GetMaxHp _unit)) 0.5))
  (|CallParentFunction))

(fn GetMovementLogic
  (return (select (Variables|Default|GethalfHealth) "NewEnumerator9" "NewEnumerator7")))

(fn CalculateSpellScoreandUpdateSpellCasting
  (params (target :type Int%20Point%20Structure) (origin :type Int%20Point%20Structure) (spell :type S%20Spell%20Data%20Structure))
  (bind _allunits (CallFunction|GetAllUnits false))
  (LocalVariables|SetallUnitsExceptSelf _allunits)
  (bind _attackedindexes (Default|GetAttackedIndexes (Variables|Default|GetcombatSystem) spell target))
  (LocalVariables|SetattackedIndexes _attackedindexes)
  (LocalVariables|SettotalSpellScore (* (* (Math|Vector|Distance2D(Vector) (Math|Conversions|ToVector2D(IntPoint) (Variables|/Game/Blueprints/Core/Units/BP_Unit.BP_Unit_C|GetIndex (Variables|Default|Getunit))) (Math|Conversions|ToVector2D(IntPoint) origin)) 1e+01) (Math|Float|SelectFloat -1.0 1.0 (Variables|Default|GethalfHealth))))
  (for _array_element (LocalVariables|GetattackedIndexes)
    (LocalVariables|SetattackedIndex _array_element)
    (if (Class|KismetMathLibrary|EqualIntPointIntPoint (LocalVariables|GetattackedIndex) origin) ; friendly fire is on and you can hurt yourself
      (LocalVariables|SetattackedUnit (Variables|Default|Getunit))
      (else
        (LocalVariables|SetattackedUnit (.Value (Utilities|Map|Find (LocalVariables|GetallUnitsExceptSelf) (LocalVariables|GetattackedIndex))))))
    (Utilities|IsValid (LocalVariables|GetattackedUnit)
      (:Is%20Valid
        (bind _impactscore (CallFunction|CalculateImpactScore spell (LocalVariables|GetattackedUnit)))
        (LocalVariables|SettotalSpellScore (+ _impactscore (LocalVariables|GettotalSpellScore))))))
  (if (> (LocalVariables|GettotalSpellScore) (Utilities|Struct|BreakS_unitAiSpellCastingData (Variables|Default|GetaiSpellCasting)))
    (Variables|Default|SetaiSpellCasting (Utilities|Struct|MakeS_unitAiSpellCastingData true (Utilities|Struct|BreakS_SpellData spell) origin target (LocalVariables|GettotalSpellScore)))))

(fn AiCombatEnded
  (|CallParentFunction))

(fn AiCombatStarted
  (|CallParentFunction))

(fn GetAvailableSpells
  ;[0 0 0] This is an example of how you can override just a sub function (It's also an easy to to tailor the spells being fed into the process)
  (return (|CallParentFunction)))